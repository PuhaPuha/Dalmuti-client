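; BP_Card is a clickable card actor that displays one of thirteen face sprites according to its Number.
; Every Tick, it switches on Number and sets the matching sprite on the Front component, polling instead of updating on change.
; Clicks on either the actor or the Front component feed a single Clicked call, with no further click logic in this graph.
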(event OnClicked(Front)
  (params (TouchedComponent :type Primitive%20Component%20Object%20Reference) (ButtonPressed :type Key%20Structure))
  (Class|Card|Clicked))

(event EventBeginPlay)

(event Collision|EventActorBeginOverlap
  (params (OtherActor :type Actor%20Object%20Reference)))

(event EventTick
  (params (DeltaSeconds :type Float%20%28single-precision%29))
  (bind _front (Variables|Default|GetFront))
  (switch int (Variables|Default|Getnumber)
    (:1
      (Rendering|Components|Sprite|SetSprite _front "/Game/Gameplay/Image/1_Sprite.1_Sprite"))
    (:2
      (Rendering|Components|Sprite|SetSprite _front "/Game/Gameplay/Image/2_Sprite.2_Sprite"))
    (:3
      (Rendering|Components|Sprite|SetSprite _front "/Game/Gameplay/Image/3_Sprite.3_Sprite"))
    (:4
      (Rendering|Components|Sprite|SetSprite _front "/Game/Gameplay/Image/4_Sprite.4_Sprite"))
    (:5
      (Rendering|Components|Sprite|SetSprite _front "/Game/Gameplay/Image/5_Sprite.5_Sprite"))
    (:6
      (Rendering|Components|Sprite|SetSprite _front "/Game/Gameplay/Image/6_Sprite.6_Sprite"))
    (:7
      (Rendering|Components|Sprite|SetSprite _front "/Game/Gameplay/Image/7_Sprite.7_Sprite"))
    (:8
      (Rendering|Components|Sprite|SetSprite _front "/Game/Gameplay/Image/8_Sprite.8_Sprite"))
    (:9
      (Rendering|Components|Sprite|SetSprite _front "/Game/Gameplay/Image/9_Sprite.9_Sprite"))
    (:10
      (Rendering|Components|Sprite|SetSprite _front "/Game/Gameplay/Image/10_Sprite.10_Sprite"))
    (:11
      (Rendering|Components|Sprite|SetSprite _front "/Game/Gameplay/Image/11_Sprite.11_Sprite"))
    (:12
      (Rendering|Components|Sprite|SetSprite _front "/Game/Gameplay/Image/12_Sprite.12_Sprite"))
    (:13
      (Rendering|Components|Sprite|SetSprite _front "/Game/Gameplay/Image/13_Sprite.13_Sprite"))))

(event MouseInput|EventActorOnClicked
  (params (ButtonPressed :type Key%20Structure))
  (Class|Card|Clicked))

(fn ConstructionScript)